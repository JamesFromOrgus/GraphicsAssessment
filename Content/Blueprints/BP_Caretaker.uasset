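; BP_Caretaker is a patrolling NPC that carries a key to be pickpocketed and restarts the level when it catches the player.
; On BeginPlay it hands its Door reference to the BP_Key in its Pickpocket child actor, then walks a looping route through TargetPoints with AI MoveTo, advancing only on successful moves.
; A first-person character overlapping its Hitbox reloads the current level.
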(event OnComponentBeginOverlap(Hitbox)
  (params (OverlappedComponent :type Primitive%20Component%20Object%20Reference) (OtherActor :type Actor%20Object%20Reference) (OtherComp :type Primitive%20Component%20Object%20Reference) (OtherBodyIndex :type Integer) (bFromSweep :type Boolean) (SweepResult :type Hit%20Result%20Structure%20%28by%20ref%29))
  (Utilities|Casting|CastToBP_FirstPersonCharacter OtherActor)
  (bind _returnvalue (Game|GetCurrentLevelName true))
  (Game|OpenLevel(byName) (Utilities|String|StringToName _returnvalue)))

(event EventBeginPlay
  (bind _targetpoints (Variables|Default|GetTargetPoints))
  (bind _asbp_key (Utilities|Casting|CastToBP_Key (Variables|/Script/Engine.ChildActorComponent|GetChildActor (Variables|Default|GetPickpocket))))
  (Variables|/Game/Blueprints/BP_Key.BP_Key_C|SetDoor _asbp_key (Variables|Default|GetDoor))
  (AI|AIMoveTo self "0, 0, 0" (Utilities|Array|Get(acopy) _targetpoints (Variables|Default|GetIndex)) 5.0 false :!label _label
    (:OnSuccess
      (Variables|Default|SetIndex (Math|Integer|%(Integer) (+ (Variables|Default|GetIndex) 1) (Utilities|Array|Length _targetpoints)))
      (goto _label))))

(fn ConstructionScript)