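; Interactable locked door that wraps a BP_BaseDoor child actor and stays shut until its HasKey flag is true.
; BeginPlay caches the child actor as the Door reference that OnInteract drives.
; Interacting while locked with the key only unlocks it; later interactions toggle the door.
; DisplayText switches between Open and Close to reflect the next available action.
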(event EventOnInteract
  (params (Interactor :type Actor%20Object%20Reference))
  (bind _door (Variables|Default|GetDoor))
  (if (Variables|Default|GetLocked)
    (if (Variables|Default|GetHasKey)
      (Variables|Default|SetLocked false)
      (Variables|Default|SetDisplayText "Open"))
    (else
      (Default|Toggle _door)
      (if (Variables|/Game/Blueprints/BP_BaseDoor.BP_BaseDoor_C|GetIsOpen _door)
        (Variables|Default|SetDisplayText "Close")
        (else
          (Variables|Default|SetDisplayText "Open"))))))

(event EventBeginPlay
  (bind _asbp_base_door (Utilities|Casting|CastToBP_BaseDoor (Variables|/Script/Engine.ChildActorComponent|GetChildActor (Variables|Default|GetChildActor))))
  (Variables|Default|SetDoor _asbp_base_door))

(fn ConstructionScript
  (|CallParentFunction))