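; BP_VentShaft is an interactable vent that moves the first-person character in and out on interaction.
; On BeginPlay it caches the VentModel from the Model child actor as the teleport reference point.
; The player's crouch state serves as the inside flag: standing players crouch and teleport above the model, crouched players stand and teleport below it.
; Each move switches the prompt between "Enter Vent" and "Exit Vent".
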(event EventBeginPlay
  (bind _asvent_model (Utilities|Casting|CastToVentModel (Variables|/Script/Engine.ChildActorComponent|GetChildActor (Variables|Default|GetModel))))
  (Variables|Default|SetVentModel _asvent_model))

(event EventOnInteract
  (params (Interactor :type Actor%20Object%20Reference))
  (bind _ventmodel (Variables|Default|GetVentModel))
  (bind _returnvalue (Transformation|GetActorLocation _ventmodel))
  (bind _asbp_first_person_character (Utilities|Casting|CastToBP_FirstPersonCharacter Interactor))
  (if (AI|Components|NavMovement|IsCrouching (Variables|/Script/Engine.Character|GetCharacterMovement _asbp_first_person_character))
    (Character|UnCrouch _asbp_first_person_character)
    (Transformation|Teleport _asbp_first_person_character (+ _returnvalue "0.000000,0.000000,-200.000000") "0, 0, 0")
    (Variables|Default|SetDisplayText "Enter Vent")
    (else
      (Character|Crouch _asbp_first_person_character)
      (Transformation|Teleport _asbp_first_person_character (+ _returnvalue "0.000000,0.000000,100.000000") "0, 0, 0")
      (Variables|Default|SetDisplayText "Exit Vent"))))

(fn ConstructionScript
  (|CallParentFunction))